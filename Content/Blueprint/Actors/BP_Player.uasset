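; Player character Blueprint that handles input, HUD creation and death, extending a parent that supplies its own death handling.
; On BeginPlay it creates the HUD for its player controller and binds health component hurt and death events, destroying itself without a controller.
; Axis inputs drive look and yaw-relative movement, and the attack action calls the weapon's Attack.
; Death runs the parent handler, then disables input.
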(event EventBeginPlay
  (bind _healthcomponent (Variables|Default|GetHealthComponent))
  (|CallParentFunction)
  (bind _asplayer_controller (Utilities|Casting|CastToPlayerController (Pawn|GetController))
    (:then
      (bind _output_get (Variables|Default|SetPlayerController _asplayer_controller))
      (bind _returnvalue (UserInterface|CreateWidget (Variables|Default|GetHudClass) _output_get))
      (UserInterface|Viewport|AddtoViewport _returnvalue 0)
      (EventDispatchers|BindEventtoOnHurt _healthcomponent (EventDispatchers|CreateEvent _returnvalue :!event SetHealth))
      (EventDispatchers|BindEventtoOnDeath _healthcomponent (EventDispatchers|CreateEvent _returnvalue :!event SetHealth)))
    (:CastFailed
      (Development|PrintString "We need a controller to make the HUD")
      (Actor|DestroyActor))))

(event Collision|EventActorBeginOverlap
  (params (OtherActor :type Actor%20Object%20Reference))
  (|CallParentFunction OtherActor) ; This node is disabled and will not be called.\nDrag off pins to build functionality.
)

(event EventTick
  (params (DeltaSeconds :type Float%20%28single-precision%29))
  (|CallParentFunction DeltaSeconds) ; This node is disabled and will not be called.\nDrag off pins to build functionality.
)

(event EventHandleDeath
  (params (Ratio :type Float%20%28single-precision%29))
  (|CallParentFunction Ratio)
  (Input|DisableInput (Variables|Default|GetPlayerController)))

(event Input|ActionEvents|InputActionAttackInput
  (params (Key :type Key%20Structure :default "None"))
  (:Pressed
    (Default|Attack (Variables|Default|GetWeapon))))

(event Input|AxisEvents|InputAxisTurnRight
  (params (AxisValue :type Float%20%28single-precision%29))
  ;[1 1 1] Comment
  ;;[1 1 1] This is the bind
  (Pawn|Input|AddControllerYawInput AxisValue))

(event Input|AxisEvents|InputAxisLookUp
  (params (AxisValue :type Float%20%28single-precision%29))
  ;[1 1 1] Comment
  (Pawn|Input|AddControllerPitchInput AxisValue))

(event Input|AxisEvents|InputAxismoveForward
  (params (AxisValue :type Float%20%28single-precision%29))
  ;[1 1 1] Comment
  ;;[1 1 1] This is the bind
  (Pawn|Input|AddMovementInput (Math|Vector|GetForwardVector (Math|Rotator|MakeRotator 0.0 0.0 (.yaw (Pawn|GetControlRotation :!class /Script/Engine.Pawn)))) AxisValue false))

(event Input|AxisEvents|InputAxisMoveRight
  (params (AxisValue :type Float%20%28single-precision%29))
  ;[1 1 1] Comment
  (Pawn|Input|AddMovementInput (Math|Vector|GetRightVector (Math|Rotator|MakeRotator 0.0 0.0 (.yaw (Pawn|GetControlRotation :!class /Script/Engine.Pawn)))) AxisValue false))

(fn ConstructionScript
  (|CallParentFunction))