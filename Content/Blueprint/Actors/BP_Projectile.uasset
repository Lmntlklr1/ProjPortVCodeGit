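; BP_Projectile is a projectile actor that deals damage to what it overlaps, then destroys itself.
; The construction script scales the collision sphere and binds its begin-overlap event.
; BeginPlay starts a one-shot timer using DestroyTimer and caches the owner, expected to be a Controller, as damage instigator.
; A component-hit event only prints a debug string.
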(event OnComponentHit(SphereCollision)
  (params (HitComponent :type Primitive%20Component%20Object%20Reference) (OtherActor :type Actor%20Object%20Reference) (OtherComp :type Primitive%20Component%20Object%20Reference) (NormalImpulse :type Vector :default "0, 0, 0") (Hit :type Hit%20Result%20Structure%20%28by%20ref%29))
  ;[1 1 1] Comment
  (Development|PrintString "Hello"))

(event Custom|HandleOverlap
  (params (OverlappedComponent :type Primitive%20Component%20Object%20Reference) (OtherActor :type Actor%20Object%20Reference) (OtherComp :type Primitive%20Component%20Object%20Reference) (OtherBodyIndex :type Integer) (bFromSweep :type Boolean) (SweepResult :type Hit%20Result%20Structure%20%28by%20ref%29))
  (Game|Damage|ApplyDamage OtherActor (Variables|Default|GetDamage) (Variables|Default|GetOwnerController) self)
  (Actor|DestroyActor))

(event EventBeginPlay
  (|CallParentFunction)
  (Utilities|Time|SetTimerbyEvent (EventDispatchers|CreateEvent :!event K2DestroyActor) (Variables|Default|GetDestroyTimer))
  (bind _ascontroller (Utilities|Casting|CastToController (Components|GetOwner))
    (:then
      (Variables|Default|SetOwnerController _ascontroller))
    (:CastFailed
      (Development|PrintString "We need the owner to be a controller"))))

(fn ConstructionScript
  (bind _spherecollision (Variables|Default|GetSphereCollision))
  (Collision|BindEventtoOnComponentBeginOverlap _spherecollision (EventDispatchers|CreateEvent :!event Custom|HandleOverlap))
  (Transformation|SetWorldScale3D _spherecollision (Variables|Default|GetScale)))