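; BP_BaseCharacter is a base character that carries a rifle and reacts to firing, hurt and death events.
; On BeginPlay it spawns the weapon class through a child actor component and caches the rifle and animation Blueprint, destroying itself if either cast fails.
; It then binds to rifle fire and health component events.
; HandleDeath plays the death animation, disables collision and notifies the weapon that its owner died.
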(event Custom|HandleDeath
  (params (Ratio :type Float%20%28single-precision%29))
  (Default|DeadAnimation (Variables|Default|GetAnimationBP) Ratio)
  (Collision|SetActorEnableCollision false)
  (Default|OwnerDied (Variables|Default|GetWeapon)))

(event EventBeginPlay
  (bind _childactorcomponent (Variables|Default|GetChildActorComponent))
  (|CallParentFunction)
  (ChildActorComponent|SetChildActorClass _childactorcomponent (Variables|Default|GetWeaponClass))
  (bind _asbp_rifle (Utilities|Casting|CastToBP_Rifle (Variables|/Script/Engine.ChildActorComponent|GetChildActor _childactorcomponent))
    (:then
      (Variables|Default|SetWeapon _asbp_rifle)
      (bind _asabp_character_animation (Utilities|Casting|CastToABP_CharacterAnimation (Components|SkeletalMesh|GetAnimInstance (Variables|Character|GetMesh)))
        (:then
          (Variables|Default|SetAnimationBP _asabp_character_animation)
          (EventDispatchers|BindEventtoOnRifleFire (Variables|Default|GetWeapon) (EventDispatchers|CreateEvent (Variables|Default|GetAnimationBP) :!event AttackAnimation))
          (EventDispatchers|BindEventtoOnHurt (Variables|Default|GetHealthComponent) (EventDispatchers|CreateEvent (Variables|Default|GetAnimationBP) :!event HurtAnimation))
          (EventDispatchers|BindEventtoOnDeath (Variables|Default|GetHealthComponent) (EventDispatchers|CreateEvent :!event Custom|HandleDeath)))
        (:CastFailed
          (Development|PrintString "We need the correct animation for the character")
          (Actor|DestroyActor))))
    (:CastFailed
      (Development|PrintString "We need a weapon for the characters ")
      (Actor|DestroyActor))))

(fn ConstructionScript)