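; Rifle actor that fires projectiles on behalf of its parent pawn, destroying itself if that parent is not a pawn.
; Attack spawns a projectile at the muzzle socket when alive and idle, starts a cooldown timer and broadcasts the fire event.
; Player aim points toward the HUD widget's EndPoint through a Blueprint-only workaround, while AI uses the pawn's base aim rotation.
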(event Custom|ActionStopped
  (Variables|Default|SetActionHappening false))

(event Custom|OwnerDied
  (Variables|Default|SetAlive false))

(event EventBeginPlay
  (bind _aspawn (Utilities|Casting|CastToPawn (Actor|GetParentActor))
    (:then
      (Variables|Default|SetParentPawn _aspawn))
    (:CastFailed
      (Development|PrintString "Rifle needs a pawn to work correctly")
      (Actor|DestroyActor))))

(fn ConstructionScript)

(fn Attack
  (bind _parentpawn (Variables|Default|GetParentPawn))
  (if (CallFunction|CanShoot)
    (Game|SpawnActorfromClass (Variables|Default|GetProjectileClass) (Math|Transform|MakeTransform (CallFunction|GetShotLocation) (CallFunction|DoNotExporttoCodeHACK) "1,1,1") "Undefined" (Pawn|GetController _parentpawn) _parentpawn)
    (Variables|Default|SetActionHappening true)
    (Utilities|Time|SetTimerbyEvent (EventDispatchers|CreateEvent :!event Custom|ActionStopped) (Variables|Default|GetShotTime))
    (Default|CallOnRifleFire)))

(fn CanShoot
  (return (and (not (Variables|Default|GetActionHappening)) (Variables|Default|GetAlive))))

(fn DoNotExporttoCodeHACK
  (bind _foundwidgets (Widget|GetAllWidgetsOfClass "/Game/Both/WBP_HUD.WBP_HUD_C" false))
  (if (== (Class|UserWidget|GetOwningPlayerPawn (Utilities|Array|Get(acopy) _foundwidgets)) (Variables|Default|GetParentPawn))
    ;[1 1 1] This is the player's Base Aim Rotation Function
    (return (Math|Rotator|MakeRotfromX (- (Variables|/Game/Both/WBP_HUD.WBP_HUD_C|GetEndPoint (Utilities|Array|Get(acopy) _foundwidgets)) (CallFunction|GetShotLocation))))
    (else
      ;[1 1 1] This is what the AI will do
      (return (Pawn|GetBaseAimRotation (Variables|Default|GetParentPawn))))))

(fn GetShotLocation
  (return (Transformation|GetSocketLocation (Variables|Default|GetSkeletalMesh) "MuzzleFlashSocket")))